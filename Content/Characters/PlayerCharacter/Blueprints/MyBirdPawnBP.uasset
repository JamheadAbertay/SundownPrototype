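; Player bird pawn Blueprint that drives flight animation and camera feedback.
; Each tick, a low DiveRangeClamped value triggers scaled camera shake and a wider, interpolated FOV.
; It feeds the NewPlayerBlue anim instance pitch from camera forward Z, plus smoothed turn and boost values.
; Turn direction comes from dotting the camera's right vector with the previous frame's forward vector, using a small dead zone.
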(event EventTick
  (params (DeltaSeconds :type Float%20%28single-precision%29))
  (bind _returnvalue (Utilities|Time|GetWorldDeltaSeconds))
  (bind _returnvalue_2 (Utilities|Time|GetWorldDeltaSeconds))
  (bind _mcamera (Variables|Default|GetmCamera))
  (bind _diverangeclamped (Variables|Default|GetDiveRangeClamped))
  (bind _mcamera_2 (Variables|Default|GetmCamera))
  (if (< _diverangeclamped 55.0)
    (Class|PlayerController|ClientPlayCameraShake (Game|GetPlayerController 0) "/Game/Characters/PlayerCharacter/Blueprints/DiveShake.DiveShake_C" (Math|Float|MapRangeClamped _diverangeclamped 75.0 5e+01 0.0 1.0) "CameraLocal" "0, 0, 0")
    ;[1 1 1] Set the DirectionZ for upward and downward animations
    (Variables|/Script/Engine.CameraComponent|SetFieldOfView _mcamera_2 (Math|Interpolation|FInterpTo (Variables|/Script/Engine.CameraComponent|GetFieldOfView _mcamera_2) 112.5 (Utilities|Time|GetWorldDeltaSeconds) 0.7))
    (else
      (Variables|/Script/Engine.CameraComponent|SetFieldOfView _mcamera_2 (Math|Interpolation|FInterpTo (Variables|/Script/Engine.CameraComponent|GetFieldOfView _mcamera_2) 105.0 (Utilities|Time|GetWorldDeltaSeconds) 0.7))))
  (bind _asnew_player_blue (Utilities|Casting|CastToNewPlayerBlue (Components|SkeletalMesh|GetAnimInstance (Variables|Character|GetMesh))))
  (Variables|/Game/Characters/NewPlayercharacter/NewPlayerBlue.NewPlayerBlue_C|SetDirectionZ _asnew_player_blue (Math|Float|Clamp(Float) (.z (Math|Vector|GetForwardVector (Variables|Default|GetmCamera))) -1.0 0.5))
  ;[1 1 1] Get the dot product of the old forward vector to the new right vector and check if character is moving left or right
  (Variables|Default|SetDirectionXYNew (Math|Vector|DotProduct (Math|Vector|GetRightVector _mcamera) (Variables|Default|GetDirectionXYPrevious)))
  (Variables|Default|SetDirectionXYPrevious (Math|Vector|GetForwardVector _mcamera))
  (if (> (Variables|Default|GetDirectionXYNew) 0.02)
    ;[1 1 1] Slowly transition to the limits of DirectionXY depending on if moving Left Right or Forward
    ;;[1 1 1] Left
    (Variables|/Game/Characters/NewPlayercharacter/NewPlayerBlue.NewPlayerBlue_C|SetDirectionXY _asnew_player_blue (Math|Interpolation|FInterpTo (Variables|/Game/Characters/NewPlayercharacter/NewPlayerBlue.NewPlayerBlue_C|GetDirectionXY _asnew_player_blue) -0.7 _returnvalue_2 1.0))
    (elif (< (Variables|Default|GetDirectionXYNew) -0.02)
      ;;[1 1 1] Right
      (Variables|/Game/Characters/NewPlayercharacter/NewPlayerBlue.NewPlayerBlue_C|SetDirectionXY _asnew_player_blue (Math|Interpolation|FInterpTo (Variables|/Game/Characters/NewPlayercharacter/NewPlayerBlue.NewPlayerBlue_C|GetDirectionXY _asnew_player_blue) 0.7 _returnvalue_2 1.0))
      (else
        ;;[1 1 1] Up and Down
        (Variables|/Game/Characters/NewPlayercharacter/NewPlayerBlue.NewPlayerBlue_C|SetDirectionXY _asnew_player_blue (Math|Interpolation|FInterpTo (Variables|/Game/Characters/NewPlayercharacter/NewPlayerBlue.NewPlayerBlue_C|GetDirectionXY _asnew_player_blue) 0.0 _returnvalue_2 3.0)))))
  (if (Variables|Default|GetBoosting)
    (Variables|/Game/Characters/NewPlayercharacter/NewPlayerBlue.NewPlayerBlue_C|SetBoosting _asnew_player_blue (Math|Interpolation|FInterpTo (Variables|/Game/Characters/NewPlayercharacter/NewPlayerBlue.NewPlayerBlue_C|GetBoosting _asnew_player_blue) 0.0 _returnvalue 3e+01))
    (else
      (Variables|/Game/Characters/NewPlayercharacter/NewPlayerBlue.NewPlayerBlue_C|SetBoosting _asnew_player_blue (Math|Interpolation|FInterpTo (Variables|/Game/Characters/NewPlayercharacter/NewPlayerBlue.NewPlayerBlue_C|GetBoosting _asnew_player_blue) 1.0 _returnvalue 2e+01)))))

(event EventBeginPlay
  ;[1 1 1] Sets the forward vector at the start of play
  (Variables|Default|SetDirectionXYPrevious (Math|Vector|GetForwardVector (Variables|Default|GetCapsuleComponent))))

(fn ConstructionScript)