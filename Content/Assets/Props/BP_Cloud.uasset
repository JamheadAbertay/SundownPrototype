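; Cloud prop that repeatedly flies along the FlightPath spline of a referenced Track actor.
; Tick uses the ActiveCloud flag as a gate, starting MoveCloud and re-arming after Duration plus CloudRestartTime.
; MoveCloud scales the timeline play rate by Duration, starts it at CloudStartOffset, and maps its Alpha to spline distance to set world location and rotation.
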(event Custom|MoveCloud
  (bind _timeline_0 (Variables|Default|GetTimeline_0))
  (bind _track (Variables|Default|GetTrack))
  (bind _flightpath (Variables|/Game/BlueprintMechanics/CreaturesSpline/SplineBirds.SplineBirds_C|GetFlightPath _track))
  (Components|Timeline|SetPlayRate _timeline_0 (/ 1.0 (Variables|Default|GetDuration)))
  (Components|Timeline|SetNewTime _timeline_0 (Variables|Default|GetCloudStartOffset))
  (bind _alpha (Timeline|Timeline_0 Play)
    (:Update
      (Variables|Default|SetAlpha _alpha)
      (Transformation|SetActorLocationAndRotation (Spline|GetLocationatDistanceAlongSpline _flightpath (Math|Float|Lerp 0.0 (Spline|GetSplineLength (Variables|/Game/BlueprintMechanics/CreaturesSpline/SplineBirds.SplineBirds_C|GetFlightPath (Variables|Default|GetTrack))) (Variables|Default|GetAlpha)) "World") (Spline|GetRotationatDistanceAlongSpline _flightpath (Math|Float|Lerp 0.0 (Spline|GetSplineLength (Variables|/Game/BlueprintMechanics/CreaturesSpline/SplineBirds.SplineBirds_C|GetFlightPath (Variables|Default|GetTrack))) (Variables|Default|GetAlpha)) "World")))))

(event Collision|EventActorBeginOverlap
  (params (OtherActor :type Actor%20Object%20Reference)))

(event EventTick
  (params (DeltaSeconds :type Float%20%28single-precision%29))
  (if (Variables|Default|GetActiveCloud)
    (CallFunction|MoveCloud)
    (Variables|Default|SetActiveCloud false)
    (Utilities|FlowControl|Delay (+ (Variables|Default|GetDuration) (Variables|Default|GetCloudRestartTime)))
    (Variables|Default|SetActiveCloud true)))

(fn ConstructionScript)