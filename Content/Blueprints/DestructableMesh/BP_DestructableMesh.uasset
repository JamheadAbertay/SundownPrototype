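; BP_DestructableMesh is a breakable prop that takes damage when the bird pawn overlaps it.
; The construction script applies the DestructableMeshForUse variable to the destructible component, so the mesh can vary.
; On overlap with MyBirdPawnBP, it checks the speed from an untargeted GetVelocity, so the prop's own rather than the bird's.
; Above a threshold, it applies damage at the component's location, with impulse direction and strength taken from that velocity.
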(event OnComponentBeginOverlap(DM_CubeTest)
  (params (OverlappedComponent :type Primitive%20Component%20Object%20Reference) (OtherActor :type Actor%20Object%20Reference) (OtherComp :type Primitive%20Component%20Object%20Reference) (OtherBodyIndex :type Integer) (bFromSweep :type Boolean) (SweepResult :type Hit%20Result%20Structure%20%28by%20ref%29))
  (bind _returnvalue (Transformation|GetVelocity))
  (bind _dm_cubetest (Variables|Default|GetDM_CubeTest))
  (bind _returnvalue_2 (Math|Vector|VectorLength _returnvalue))
  (Utilities|Casting|CastToMyBirdPawnBP OtherActor)
  (if (> _returnvalue_2 2e+02)
    (Class|DestructibleComponent|ApplyDamage _dm_cubetest 1.0 (Transformation|GetWorldLocation _dm_cubetest) _returnvalue _returnvalue_2)))

(event EventBeginPlay)

(event Collision|EventActorBeginOverlap
  (params (OtherActor :type Actor%20Object%20Reference)))

(event EventTick
  (params (DeltaSeconds :type Float%20%28single-precision%29)))

(fn ConstructionScript
  (Class|DestructibleComponent|SetDestructibleMesh (Variables|Default|GetDM_CubeTest) (Variables|Default|GetDestructableMeshForUse)))