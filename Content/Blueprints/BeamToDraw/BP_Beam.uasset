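; BP_Beam is a placeable beam actor with a cylinder mesh and a sphere trigger that toggles the beam's visibility.
; The construction script applies an exposed material and sets cylinder and trigger scales from BeamSize and CollisionSize.
; Sphere overlap hides the cylinder on entry and shows it on exit.
; Both events require the overlapping actor to cast to PlayerController, so an ordinary player Pawn does not pass the check.
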(event OnComponentBeginOverlap(Sphere)
  (params (OverlappedComponent :type Primitive%20Component%20Object%20Reference) (OtherActor :type Actor%20Object%20Reference) (OtherComp :type Primitive%20Component%20Object%20Reference) (OtherBodyIndex :type Integer) (bFromSweep :type Boolean) (SweepResult :type Hit%20Result%20Structure%20%28by%20ref%29))
  (Utilities|Casting|CastToPlayerController OtherActor)
  (Rendering|SetVisibility (Variables|Default|GetCylinder1) false false))

(event OnComponentEndOverlap(Sphere)
  (params (OverlappedComponent :type Primitive%20Component%20Object%20Reference) (OtherActor :type Actor%20Object%20Reference) (OtherComp :type Primitive%20Component%20Object%20Reference) (OtherBodyIndex :type Integer))
  (Utilities|Casting|CastToPlayerController OtherActor)
  (Rendering|SetVisibility (Variables|Default|GetCylinder1) true false))

(event EventBeginPlay)

(event Collision|EventActorBeginOverlap
  (params (OtherActor :type Actor%20Object%20Reference)))

(event EventTick
  (params (DeltaSeconds :type Float%20%28single-precision%29)))

(fn ConstructionScript
  (Rendering|Material|SetMaterial (Variables|Default|GetCylinder1) 0 (Variables|Default|GetMaterial))
  (Transformation|SetRelativeScale3D (Variables|Default|GetSphere) (Variables|Default|GetCollisionSize))
  (Transformation|SetRelativeScale3D (Variables|Default|GetCylinder1) (Variables|Default|GetBeamSize)))