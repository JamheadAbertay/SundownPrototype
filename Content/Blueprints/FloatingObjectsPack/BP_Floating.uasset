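; Floating manager Blueprint that bobs an array of actors up and down on a looping timeline.
; Construction script caches each actor's original location.
; BeginPlay sets timeline rate from float duration and plays if enabled; finishing restarts it.
; Each update sets root locations through FloatingMovement, whose Z-lerp around the cached location appears unconnected.
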(event Custom|Float
  (Components|Timeline|SetPlayRate (Variables|Default|GetFloatingSpeed) (/ 1.0 (Variables|Default|GetHow%20long%20to%20complete%201%20float)))
  (if (Variables|Default|GetShouldFloat?)
    (bind _floatspeed (Timeline|FloatingSpeed Play)
      (:Update
        (for (_array_element _array_index) (Variables|Default|GetArrayOfObjectsToFloat)
          (Transformation|SetWorldLocation (Variables|/Script/Engine.Actor|GetRootComponent _array_element) (Utilities|FloatingMovement _array_index _floatspeed) false false)))
      (:Finished
        (CallFunction|RestartTrack)))))

(event Custom|RestartTrack
  (bind _floatspeed (Timeline|FloatingSpeed PlayFromStart)
    (:Update
      (for (_array_element _array_index) (Variables|Default|GetArrayOfObjectsToFloat)
        (Transformation|SetWorldLocation (Variables|/Script/Engine.Actor|GetRootComponent _array_element) (Utilities|FloatingMovement _array_index _floatspeed) false false)))
    (:Finished
      (CallFunction|RestartTrack))))

(event EventBeginPlay
  (CallFunction|Float))

(fn ConstructionScript
  (for (_array_element _array_index) (Variables|Default|GetArrayOfObjectsToFloat)
    (Utilities|Array|SetArrayElem (Variables|Default|GetOriginalLocation) _array_index (Transformation|GetActorLocation _array_element) true)))