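; Creature actor that flies a bird along the FlightPath spline of a referenced Track, repeating after a pause.
; Construction script applies the configurable static mesh, material and skeletal mesh; BeginPlay sets the anim class, then plays a looping animation.
; Tick uses the ActiveBird flag and a Delay to retrigger the BirdFlight timeline, scaled to Duration and started at an offset.
; Timeline alpha maps to spline distance, setting world location and rotation.
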(event Custom|MoveBird
  (bind _birdflight (Variables|Default|GetBirdFlight))
  (bind _track (Variables|Default|GetTrack))
  (bind _flightpath (Variables|/Game/Blueprints/CreaturesSpline/SplineBirds.SplineBirds_C|GetFlightPath _track))
  (Components|Timeline|SetPlayRate _birdflight (/ 1.0 (Variables|Default|GetDuration)))
  (Components|Timeline|SetNewTime _birdflight (Variables|Default|GetBirdStartOffset))
  (bind _alpha (Timeline|BirdFlight Play)
    (:Update
      (Variables|Default|SetAlpha _alpha)
      (Transformation|SetActorLocationAndRotation (Spline|GetLocationatDistanceAlongSpline _flightpath (Math|Float|Lerp 0.0 (Spline|GetSplineLength (Variables|/Game/Blueprints/CreaturesSpline/SplineBirds.SplineBirds_C|GetFlightPath (Variables|Default|GetTrack))) (Variables|Default|GetAlpha)) "World") (Spline|GetRotationatDistanceAlongSpline _flightpath (Math|Float|Lerp 0.0 (Spline|GetSplineLength (Variables|/Game/Blueprints/CreaturesSpline/SplineBirds.SplineBirds_C|GetFlightPath (Variables|Default|GetTrack))) (Variables|Default|GetAlpha)) "World")))))

(event EventBeginPlay
  (Components|SkeletalMesh|SetAnimInstanceClass (Variables|Default|GetSkeletalMesh) (Utilities|GetClass (Variables|Default|GetAnimationBP)))
  (Components|Animation|PlayAnimation (Variables|Default|GetSkeletalMesh) (.AnimToPlay (Utilities|Struct|BreakSingleAnimationPlayData (Variables|Default|GetAnimation))) true))

(event EventTick
  (params (DeltaSeconds :type Float%20%28single-precision%29))
  (if (Variables|Default|GetActiveBird)
    (CallFunction|MoveBird)
    (Variables|Default|SetActiveBird false)
    (Utilities|FlowControl|Delay (+ (Variables|Default|GetDuration) (Variables|Default|GetBirdRestartTime)))
    (Variables|Default|SetActiveBird true)))

(fn ConstructionScript
  (bind _staticmesh (Variables|Default|GetStaticMesh))
  (Components|StaticMesh|SetStaticMesh _staticmesh (Variables|Default|GetCurrentMesh))
  (Rendering|Material|SetMaterial _staticmesh 0 (Variables|Default|GetMaterialOfStatic))
  (Class|SkinnedMeshComponent|SetSkeletalMesh (Variables|Default|GetSkeletalMesh) (Variables|Default|GetSkeletonMesh) true))