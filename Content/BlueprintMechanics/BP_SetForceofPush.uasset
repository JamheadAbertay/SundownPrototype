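; BP_SetForceofPush is a level-wide configuration actor that applies one shared ForceOfCollisionPush value to the six directional push actor types.
; On BeginPlay it finds all Right, Down, Forward, Left, Back and Up push actors and overwrites each one's force amount.
; The loops are nested in that order, so later types are reassigned repeatedly and are skipped if an earlier type has no instances.
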(event EventBeginPlay
  (bind _forceofcollisionpush (Variables|Default|GetForceOfCollisionPush))
  (bind _outactors (Actor|GetAllActorsOfClass "/Game/BlueprintMechanics/BP_PushRight.BP_PushRight_C"))
  (for _array_element _outactors
    (Variables|/Game/BlueprintMechanics/BP_PushRight.BP_PushRight_C|SetRightForceAmount _array_element _forceofcollisionpush)
    (bind _outactors_2 (Actor|GetAllActorsOfClass "/Game/BlueprintMechanics/BP_PushDown.BP_PushDown_C"))
    (for _array_element_2 _outactors_2
      (Variables|/Game/BlueprintMechanics/BP_PushDown.BP_PushDown_C|SetDown%20Force%20Amount _array_element_2 _forceofcollisionpush)
      (bind _outactors_3 (Actor|GetAllActorsOfClass "/Game/BlueprintMechanics/BP_PushForward.BP_PushForward_C"))
      (for _array_element_3 _outactors_3
        (Variables|/Game/BlueprintMechanics/BP_PushForward.BP_PushForward_C|SetForward%20Force%20Amount _array_element_3 _forceofcollisionpush)
        (bind _outactors_4 (Actor|GetAllActorsOfClass "/Game/BlueprintMechanics/BP_PushLeft.BP_PushLeft_C"))
        (for _array_element_4 _outactors_4
          (Variables|/Game/BlueprintMechanics/BP_PushLeft.BP_PushLeft_C|SetLeftForceAmount _array_element_4 _forceofcollisionpush)
          (bind _outactors_5 (Actor|GetAllActorsOfClass "/Game/BlueprintMechanics/BP_PushBack.BP_PushBack_C"))
          (for _array_element_5 _outactors_5
            (Variables|/Game/BlueprintMechanics/BP_PushBack.BP_PushBack_C|SetBackForceAmount _array_element_5 _forceofcollisionpush)
            (bind _outactors_6 (Actor|GetAllActorsOfClass "/Game/BlueprintMechanics/BP_PushUp.BP_PushUp_C"))
            (for _array_element_6 _outactors_6
              (Variables|/Game/BlueprintMechanics/BP_PushUp.BP_PushUp_C|SetUp%20Force%20Amount _array_element_6 _forceofcollisionpush))))))))

(fn ConstructionScript)