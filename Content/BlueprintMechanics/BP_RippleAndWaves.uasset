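; BP_RippleAndWaves is a spline-driven actor that lays a chain of deformed meshes along RippleSpline, presumably for ripple or wave shapes.
; Its construction script adds one spline mesh per segment, attached to RailSystem and bent using the local locations and tangents of adjacent points.
; RelativScale sizes each new mesh and is also applied to the spline itself.
; The event graph has no active logic.
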(event EventBeginPlay)

(event Collision|EventActorBeginOverlap
  (params (OtherActor :type Actor%20Object%20Reference)))

(event EventTick
  (params (DeltaSeconds :type Float%20%28single-precision%29)))

(fn ConstructionScript
  (bind _relativscale (Variables|Default|GetRelativScale))
  (bind _ripplespline (Variables|Default|GetRippleSpline))
  (for _index (range 0 (- (Spline|GetNumberOfSplinePoints (Variables|Default|GetRippleSpline)) 2))
    (bind _returnvalue (AddComponent|AddSplineMeshComponent true (Math|Transform|MakeTransform "0, 0, 0" "0, 0, 0" _relativscale)))
    (Transformation|SetRelativeScale3D (Variables|Default|GetRippleSpline) _relativscale)
    (Transformation|AttachComponentToComponent _returnvalue (Variables|Default|GetRailSystem) "None" "KeepRelative" "KeepRelative" "KeepRelative" true)
    (SplineMesh|SetStartandEnd _returnvalue (.Location (Spline|GetLocationandTangentatSplinePoint _ripplespline _index "Local")) (.Tangent (Spline|GetLocationandTangentatSplinePoint _ripplespline _index "Local")) (.Location (Spline|GetLocationandTangentatSplinePoint _ripplespline (+ _index 1) "Local")) (.Tangent (Spline|GetLocationandTangentatSplinePoint _ripplespline (+ _index 1) "Local")) true :!class /Script/Engine.SplineMeshComponent)))