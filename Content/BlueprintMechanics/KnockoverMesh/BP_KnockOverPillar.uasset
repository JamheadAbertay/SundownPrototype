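; BP_KnockOverPillar is a destructible pillar that breaks when a BP_Armadillo hits it fast enough.
; A hidden CollisionArea destructible detects overlaps and, above a speed threshold, applies damage to DMCubeTest with an impulse along the armadillo's velocity, scaled by its speed.
; The construction script assigns a configurable destructible mesh to both components, then scales, offsets and gives an outline material to the collision copy.
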(event OnComponentBeginOverlap(CollisionArea)
  (params (OverlappedComponent :type Primitive%20Component%20Object%20Reference) (OtherActor :type Actor%20Object%20Reference) (OtherComp :type Primitive%20Component%20Object%20Reference) (OtherBodyIndex :type Integer) (bFromSweep :type Boolean) (SweepResult :type Hit%20Result%20Structure%20%28by%20ref%29))
  (bind _dm_cubetest (Variables|Default|GetDM_CubeTest))
  (bind _asbp_armadillo (Utilities|Casting|CastToBP_Armadillo OtherActor))
  (if (> (Math|Vector|VectorLength (Transformation|GetVelocity _asbp_armadillo)) 1.5e+03)
    (Class|DestructibleComponent|ApplyDamage _dm_cubetest 1.0 (Transformation|GetWorldLocation _dm_cubetest) (Transformation|GetVelocity _asbp_armadillo) (Math|Vector|VectorLength (Transformation|GetVelocity _asbp_armadillo)))))

(event EventBeginPlay)

(event Collision|EventActorBeginOverlap
  (params (OtherActor :type Actor%20Object%20Reference)))

(event EventTick
  (params (DeltaSeconds :type Float%20%28single-precision%29)))

(fn ConstructionScript
  (bind _collisionarea (Variables|Default|GetCollisionArea))
  (Class|DestructibleComponent|SetDestructibleMesh (Variables|Default|GetDM_CubeTest) (Variables|Default|GetDestructableMeshForUse))
  (Class|DestructibleComponent|SetDestructibleMesh _collisionarea (Variables|Default|GetDestructableMeshForUse))
  (Transformation|SetRelativeScale3D _collisionarea (Variables|Default|GetCollision%20Scale))
  (Transformation|AddLocalOffset _collisionarea (Variables|Default|GetCollision%20Offset) false false)
  (Rendering|Material|SetMaterial _collisionarea 0 "/Game/BlueprintMechanics/DestructableMesh/MI_CollisionMeshOutline.MI_CollisionMeshOutline")
  (Development|SetHiddeninGame _collisionarea true false))