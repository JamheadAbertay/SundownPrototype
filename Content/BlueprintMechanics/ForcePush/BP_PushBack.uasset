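; Trigger-box actor that pushes the bird pawn back along Y and turns it around when it enters the volume.
; Overlap stores the pawn and its entry Y; Tick then applies a movement force scaled by its Y offset from that point.
; While inside, pawn input is disabled and control yaw interpolates toward 270 degrees.
; Outside, Tick re-enables player character input every frame.
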(event OnComponentBeginOverlap(Box)
  (params (OverlappedComponent :type Primitive%20Component%20Object%20Reference) (OtherActor :type Actor%20Object%20Reference) (OtherComp :type Primitive%20Component%20Object%20Reference) (OtherBodyIndex :type Integer) (bFromSweep :type Boolean) (SweepResult :type Hit%20Result%20Structure%20%28by%20ref%29))
  (bind _asmy_bird_pawn_bp (Utilities|Casting|CastToMyBirdPawnBP OtherActor))
  (Variables|Default|SetCharacterControllerRotationOn? true)
  (Variables|Default|SetYValueWhenGoIn (.y (Transformation|GetActorLocation _asmy_bird_pawn_bp)))
  (Variables|Default|SetInBox true))

(event OnComponentEndOverlap(Box)
  (params (OverlappedComponent :type Primitive%20Component%20Object%20Reference) (OtherActor :type Actor%20Object%20Reference) (OtherComp :type Primitive%20Component%20Object%20Reference) (OtherBodyIndex :type Integer))
  (Variables|Default|SetInBox false)
  (Variables|Default|SetCharacterControllerRotationOn? false))

(event EventTick
  (params (DeltaSeconds :type Float%20%28single-precision%29))
  (bind _returnvalue (Game|GetPlayerController 0))
  (if (Variables|Default|GetCharacterControllerRotationOn?)
    (Input|DisableInput (stale OnComponentBeginOverlap(Box) _asmy_bird_pawn_bp) _returnvalue)
    (else
      (Input|EnableInput (Game|GetPlayerCharacter 0) _returnvalue)))
  (if (Variables|Default|GetInBox)
    (bind _output_get (Variables|Default|SetYValueCurrent (.y (Transformation|GetActorLocation (stale OnComponentBeginOverlap(Box) _asmy_bird_pawn_bp)))))
    (Physics|AddForce (Variables|/Script/Engine.Character|GetCharacterMovement (stale OnComponentBeginOverlap(Box) _asmy_bird_pawn_bp)) (* (Math|Vector|MakeVector 0.0 (Variables|Default|GetBackForceAmount) 0.0) (- _output_get (Variables|Default|GetYValueWhenGoIn))))
    (if (or (>= (.yaw (Pawn|GetControlRotation (stale OnComponentBeginOverlap(Box) _asmy_bird_pawn_bp) :!class /Script/Engine.Pawn)) 270.5) (< (.yaw (Pawn|GetControlRotation (stale OnComponentBeginOverlap(Box) _asmy_bird_pawn_bp) :!class /Script/Engine.Pawn)) 269.5))
      (Pawn|SetControlRotation (Game|GetPlayerController 0) (Math|Rotator|MakeRotator (.roll (Pawn|GetControlRotation (stale OnComponentBeginOverlap(Box) _asmy_bird_pawn_bp) :!class /Script/Engine.Pawn)) (.pitch (Pawn|GetControlRotation (stale OnComponentBeginOverlap(Box) _asmy_bird_pawn_bp) :!class /Script/Engine.Pawn)) (Math|Interpolation|FInterpTo (.yaw (Pawn|GetControlRotation (stale OnComponentBeginOverlap(Box) _asmy_bird_pawn_bp) :!class /Script/Engine.Pawn)) 2.7e+02 (Utilities|Time|GetWorldDeltaSeconds) 1.2))))))

(fn ConstructionScript)