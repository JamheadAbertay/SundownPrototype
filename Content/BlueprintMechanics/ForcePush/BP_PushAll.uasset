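; BP_PushAll is a box volume that pushes the player's bird back toward where it entered.
; On overlap it stores the entry location and disables bird input until an overlap ends.
; Each tick inside, it adds per-axis, spring-like force to player character movement, proportional to the offset from entry.
; Control-rotation helper functions are never called; only RotateRight (pitch) and RotateBack (yaw) contain interpolation logic.
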(event OnComponentBeginOverlap(Box)
  (params (OverlappedComponent :type Primitive%20Component%20Object%20Reference) (OtherActor :type Actor%20Object%20Reference) (OtherComp :type Primitive%20Component%20Object%20Reference) (OtherBodyIndex :type Integer) (bFromSweep :type Boolean) (SweepResult :type Hit%20Result%20Structure%20%28by%20ref%29))
  (bind _asmy_bird_pawn_bp (Utilities|Casting|CastToMyBirdPawnBP OtherActor))
  (Variables|Default|SetCharacterControllerRotationOn? true)
  (Variables|Default|SetXValueAtEntry (.x (Transformation|GetActorLocation _asmy_bird_pawn_bp)))
  (Variables|Default|SetYValueAtEntry (.y (Transformation|GetActorLocation _asmy_bird_pawn_bp)))
  (Variables|Default|SetZValueAtEntry (.z (Transformation|GetActorLocation _asmy_bird_pawn_bp)))
  (Variables|Default|SetInBox true))

(event OnComponentEndOverlap(Box)
  (params (OverlappedComponent :type Primitive%20Component%20Object%20Reference) (OtherActor :type Actor%20Object%20Reference) (OtherComp :type Primitive%20Component%20Object%20Reference) (OtherBodyIndex :type Integer))
  (Variables|Default|SetInBox false)
  (Variables|Default|SetCharacterControllerRotationOn? false))

(event EventTick
  (params (DeltaSeconds :type Float%20%28single-precision%29))
  (bind _returnvalue (Game|GetPlayerController 0))
  (if (Variables|Default|GetCharacterControllerRotationOn?)
    (Input|DisableInput (stale OnComponentBeginOverlap(Box) _asmy_bird_pawn_bp) _returnvalue)
    (else
      (Input|EnableInput (Game|GetPlayerCharacter 0) _returnvalue)))
  (if (Variables|Default|GetInBox)
    (Variables|Default|SetXValueAtCurrent (.x (Transformation|GetActorLocation (stale OnComponentBeginOverlap(Box) _asmy_bird_pawn_bp))))
    (Variables|Default|SetYValueAtCurrent (.y (Transformation|GetActorLocation (stale OnComponentBeginOverlap(Box) _asmy_bird_pawn_bp))))
    (Variables|Default|SetZValueAtCurrent (.z (Transformation|GetActorLocation (stale OnComponentBeginOverlap(Box) _asmy_bird_pawn_bp))))
    (CallFunction|AddingForcetoPlayer (Variables|Default|GetXValueAtEntry) (Variables|Default|GetXValueAtCurrent) (Variables|Default|GetForceAmount) 0.0 0.0)
    (CallFunction|AddingForcetoPlayer (Variables|Default|GetYValueAtEntry) (Variables|Default|GetYValueAtCurrent) 0.0 (Variables|Default|GetForceAmount) 0.0)
    (CallFunction|AddingForcetoPlayer (Variables|Default|GetZValueAtEntry) (Variables|Default|GetZValueAtCurrent) 0.0 0.0 (Variables|Default|GetForceAmount))
    (if (< (Variables|Default|GetXValueAtEntry) (Variables|Default|GetXValueAtCurrent))
      _)))

(fn ConstructionScript)

(fn AddingForcetoPlayer
  (params (ValueAtEntry :type Float%20%28single-precision%29) (ValueAtCurrent :type Float%20%28single-precision%29) (XForceAmount :type Float%20%28single-precision%29) (YForceAmount :type Float%20%28single-precision%29) (ZForceAmount :type Float%20%28single-precision%29))
  (Physics|AddForce (Variables|/Script/Engine.Character|GetCharacterMovement (Game|GetPlayerCharacter 0)) (* (Math|Vector|MakeVector XForceAmount YForceAmount ZForceAmount) (- ValueAtEntry ValueAtCurrent))))

(fn RotateRight
  (params (PlayerCharacter :type Pawn%20Object%20Reference) (PlayerController :type Player%20Controller%20Object%20Reference))
  (bind _returnvalue (Pawn|GetControlRotation PlayerCharacter :!class /Script/Engine.Pawn))
  (if (>= (.pitch _returnvalue) 1.0)
    (Pawn|SetControlRotation PlayerController (Math|Rotator|MakeRotator (.roll _returnvalue) (Math|Interpolation|FInterpTo (.pitch _returnvalue) 0.0 (Utilities|Time|GetWorldDeltaSeconds) 2.6) (.yaw _returnvalue)))))

(fn RotateLeft)

(fn RotateDown)

(fn RotateUp)

(fn RotateForward
  (params (PlayerCharacter :type Pawn%20Object%20Reference) (PlayerController :type Player%20Controller%20Object%20Reference)))

(fn RotateBack
  (params (PlayerCharacter :type Pawn%20Object%20Reference) (PlayerController :type Player%20Controller%20Object%20Reference))
  (bind _returnvalue (Pawn|GetControlRotation PlayerCharacter :!class /Script/Engine.Pawn))
  (if (or (>= (.yaw _returnvalue) 270.5) (< (.yaw _returnvalue) 269.5))
    (Pawn|SetControlRotation PlayerController (Math|Rotator|MakeRotator (.roll _returnvalue) (.pitch _returnvalue) (Math|Interpolation|FInterpTo (.yaw _returnvalue) 2.7e+02 (Utilities|Time|GetWorldDeltaSeconds) 1.2)))))