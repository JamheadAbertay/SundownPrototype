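; BP_PushLeft is a force volume that pushes the bird pawn along the world X axis, presumably leftward as named.
; Box overlap caches the MyBirdPawnBP and its entry X, and any end overlap switches the push off.
; While active, Tick adds LeftForceAmount through CharacterMovement, scaled by the pawn's X distance from its entry point.
; A disconnected control-pitch interpolation never runs.
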(event OnComponentBeginOverlap(Box)
  (params (OverlappedComponent :type Primitive%20Component%20Object%20Reference) (OtherActor :type Actor%20Object%20Reference) (OtherComp :type Primitive%20Component%20Object%20Reference) (OtherBodyIndex :type Integer) (bFromSweep :type Boolean) (SweepResult :type Hit%20Result%20Structure%20%28by%20ref%29))
  (bind _asmy_bird_pawn_bp (Utilities|Casting|CastToMyBirdPawnBP OtherActor))
  (Variables|Default|SetXValueWhenGoIn (.x (Transformation|GetActorLocation _asmy_bird_pawn_bp)))
  (Variables|Default|SetInBox true))

(event OnComponentEndOverlap(Box)
  (params (OverlappedComponent :type Primitive%20Component%20Object%20Reference) (OtherActor :type Actor%20Object%20Reference) (OtherComp :type Primitive%20Component%20Object%20Reference) (OtherBodyIndex :type Integer))
  (Variables|Default|SetInBox false))

(event EventBeginPlay)

(event Collision|EventActorBeginOverlap
  (params (OtherActor :type Actor%20Object%20Reference)))

(event EventTick
  (params (DeltaSeconds :type Float%20%28single-precision%29))
  (if (Variables|Default|GetInBox)
    (bind _output_get (Variables|Default|SetXValueCurrent (.x (Transformation|GetActorLocation (stale OnComponentBeginOverlap(Box) _asmy_bird_pawn_bp)))))
    (Physics|AddForce (Variables|/Script/Engine.Character|GetCharacterMovement (stale OnComponentBeginOverlap(Box) _asmy_bird_pawn_bp)) (* (Math|Vector|MakeVector (Variables|Default|GetLeftForceAmount) 0.0 0.0) (Math|Float|Absolute(Float) (- (* _output_get -1.0) (* (Variables|Default|GetXValueWhenGoIn) -1.0)))))))

(fn ConstructionScript)