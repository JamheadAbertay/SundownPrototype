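; Trigger volume that pushes the player's bird pawn forward along world +Y while it is inside the box.
; On overlap it records the entry Y, then Tick applies movement force scaled by distance from that point and eases control yaw toward +Y.
; Player input is disabled during the push and restored shortly after exit; Tick reapplies this input state every frame.
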(event OnComponentBeginOverlap(Box)
  (params (OverlappedComponent :type Primitive%20Component%20Object%20Reference) (OtherActor :type Actor%20Object%20Reference) (OtherComp :type Primitive%20Component%20Object%20Reference) (OtherBodyIndex :type Integer) (bFromSweep :type Boolean) (SweepResult :type Hit%20Result%20Structure%20%28by%20ref%29))
  (bind _asmy_bird_pawn_bp (Utilities|Casting|CastToMyBirdPawnBP OtherActor))
  (Variables|Default|SetCharacterRotationOff true)
  (Variables|Default|SetYValueWhenGoIn (.y (Transformation|GetActorLocation _asmy_bird_pawn_bp)))
  (Variables|Default|SetInBox true))

(event OnComponentEndOverlap(Box)
  (params (OverlappedComponent :type Primitive%20Component%20Object%20Reference) (OtherActor :type Actor%20Object%20Reference) (OtherComp :type Primitive%20Component%20Object%20Reference) (OtherBodyIndex :type Integer))
  (Variables|Default|SetInBox false)
  (Utilities|FlowControl|Delay 0.05)
  (Variables|Default|SetCharacterRotationOff false))

(event EventTick
  (params (DeltaSeconds :type Float%20%28single-precision%29))
  (bind _returnvalue (Game|GetPlayerController 0))
  (bind _returnvalue_2 (Game|GetPlayerCharacter 0))
  (if (Variables|Default|GetCharacterRotationOff)
    (Input|DisableInput _returnvalue_2 _returnvalue)
    (else
      (Input|EnableInput _returnvalue_2 _returnvalue)))
  (if (Variables|Default|GetInBox)
    (bind _output_get (Variables|Default|SetYValueCurrent (.y (Transformation|GetActorLocation (stale OnComponentBeginOverlap(Box) _asmy_bird_pawn_bp)))))
    (Physics|AddForce (Variables|/Script/Engine.Character|GetCharacterMovement (stale OnComponentBeginOverlap(Box) _asmy_bird_pawn_bp)) (* (Math|Vector|MakeVector 0.0 (Variables|Default|GetForward%20Force%20Amount) 0.0) (Math|Float|Absolute(Float) (- _output_get (Variables|Default|GetYValueWhenGoIn)))))
    (Pawn|SetControlRotation (Game|GetPlayerController 0) (Math|Rotator|MakeRotator (.roll (Pawn|GetControlRotation (stale OnComponentBeginOverlap(Box) _asmy_bird_pawn_bp) :!class /Script/Engine.Pawn)) (.pitch (Pawn|GetControlRotation (stale OnComponentBeginOverlap(Box) _asmy_bird_pawn_bp) :!class /Script/Engine.Pawn)) (Math|Interpolation|FInterpTo (.yaw (Pawn|GetControlRotation (stale OnComponentBeginOverlap(Box) _asmy_bird_pawn_bp) :!class /Script/Engine.Pawn)) 9e+01 (Utilities|Time|GetWorldDeltaSeconds) 1.2)))))

(fn ConstructionScript)