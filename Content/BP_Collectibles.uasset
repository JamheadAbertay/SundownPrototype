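; BP_Collectibles is a spinning pickup actor that adds to the player's CollectibleEye count.
; Overlap by the bird pawn, third-person character or armadillo increments the counter in the GI_Sundown game instance, then destroys the pickup.
; The construction script applies a configurable mesh.
; Tick adds a local rotation derived from the RotationSpeed vector as an X axis, without delta-time scaling.
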(event EventBeginPlay)

(event Collision|EventActorBeginOverlap
  (params (OtherActor :type Actor%20Object%20Reference))
  (bind _returnvalue (Game|GetGameInstance))
  (bind _asgi_sundown (Utilities|Casting|CastToGI_Sundown _returnvalue))
  (Utilities|Casting|CastToMyBirdPawnBP OtherActor
    (:then
      _)
    (:CastFailed
      (Utilities|Casting|CastToThirdPersonCharacter OtherActor
        (:then
          _)
        (:CastFailed
          (Utilities|Casting|CastToBP_Armadillo OtherActor)))))
  (Variables|/Game/GI_Sundown.GI_Sundown_C|SetCollectibleEye _asgi_sundown (+ (Variables|/Game/GI_Sundown.GI_Sundown_C|GetCollectibleEye _asgi_sundown) 1.0))
  (Actor|DestroyActor))

(event EventTick
  (params (DeltaSeconds :type Float%20%28single-precision%29))
  (Transformation|AddLocalRotation (Variables|Default|GetStaticMesh) (Math|Conversions|RotationFromXVector (Variables|CollectibleSettings|GetRotationSpeed)) false false))

(fn ConstructionScript
  (Components|StaticMesh|SetStaticMesh (Variables|Default|GetStaticMesh) (Variables|CollectibleSettings|GetCollectibleMesh)))