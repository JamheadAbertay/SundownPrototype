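; BP_BellTrigger is a sphere trigger that rings a bell-style cue when the player's bird pawn flies into it.
; On overlap by MyBirdPawnBP, a DoOnce gate plays a 2D sound and creates and plays a level sequence player from the assigned sequence and settings.
; When the bird leaves the sphere, the gate resets only if Repeatable is set, allowing one-shot or repeatable triggers.
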(event OnComponentBeginOverlap(Sphere)
  (params (OverlappedComponent :type Primitive%20Component%20Object%20Reference) (OtherActor :type Actor%20Object%20Reference) (OtherComp :type Primitive%20Component%20Object%20Reference) (OtherBodyIndex :type Integer) (bFromSweep :type Boolean) (SweepResult :type Hit%20Result%20Structure%20%28by%20ref%29))
  (Utilities|Casting|CastToMyBirdPawnBP OtherActor)
  (Utilities|FlowControl|DoOnce false
    (:Completed
      (bind _outactor (Sequencer|Player|CreateLevelSequencePlayer (Variables|Default|GetSequence) (Variables|Default|GetPlaySettings)))
      (Audio|PlaySound2D (Variables|Default|GetSoundToPlay))
      (Sequencer|Player|Play (Variables|/Script/LevelSequence.LevelSequenceActor|GetSequencePlayer _outactor) :!class /Script/MovieScene.MovieSceneSequencePlayer))))

(event OnComponentEndOverlap(Sphere)
  (params (OverlappedComponent :type Primitive%20Component%20Object%20Reference) (OtherActor :type Actor%20Object%20Reference) (OtherComp :type Primitive%20Component%20Object%20Reference) (OtherBodyIndex :type Integer))
  (Utilities|Casting|CastToMyBirdPawnBP OtherActor)
  (if (Variables|Default|GetRepeatable)
    (Utilities|FlowControl|DoOnce false) ; enters at Reset
  ))

(fn ConstructionScript)